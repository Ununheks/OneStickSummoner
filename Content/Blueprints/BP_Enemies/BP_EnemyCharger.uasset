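; BP_EnemyCharger is an enemy that chases the player on sight and deals contact damage.
; Pawn sensing starts an AI move toward any seen TwinStickPawn.
; Capsule hits on actors tagged Player apply fixed damage, gated by a cooldown of one over AttackDelay, so that variable acts as a rate.
; Incoming damage lowers health and destroys the enemy once it drops below zero.
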(event `self.PawnSensing.OnSeePawn`
  (params (Pawn :type "Pawn Object Reference"))
  ;[1 1 1] Move towards a player when it sees him
  (bind _astwin_stick_pawn (cast `/Game/TwinStickBP/Blueprints/TwinStickPawn` Pawn))
  (`|AIMoveTo` self (0.0 0.0 0.0) _astwin_stick_pawn))

(event `self.ReceiveAnyDamage`
  (params (Damage :type "Float (single-precision)") (DamageType :type "DamageType Object Reference") (InstigatedBy :type "Controller Object Reference") (DamageCauser :type "Actor Object Reference"))
  ;[1 1 1] Getting damaged
  (set `self.CurrentHealth` (- (`self.CurrentHealth`) Damage))
  (if (< (`self.CurrentHealth`) 0.0)
    (set `self.isDead?` true)
    (`self.K2_DestroyActor`)))

(event `self.CapsuleComponent.OnComponentHit`
  (params (HitComponent :type "PrimitiveComponent Object Reference") (OtherActor :type "Actor Object Reference") (OtherComp :type "PrimitiveComponent Object Reference") (NormalImpulse :type "Vector Structure") (Hit :type "HitResult Structure (by ref)"))
  ;[1 1 1] Damaging player by hitting him
  (if (`self.canAtack?`)
    (if (`self.ActorHasTag` OtherActor "Player")
      (`GameplayStatics.ApplyDamage` OtherActor 10.0)
      (set `self.canAtack?` false)
      (`KismetSystemLibrary.Delay` (/ 1.0 (`self.AttackDelay`)))
      (set `self.canAtack?` true))))

(fn `UserConstructionScript`)