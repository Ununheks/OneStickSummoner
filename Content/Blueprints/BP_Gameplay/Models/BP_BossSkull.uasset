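; BP_BossSkull is a boss skull model that periodically turns its Cube component to face the player's camera.
; On BeginPlay it caches player 0's pawn as a TwinStickPawn and, if the cast succeeds, starts a looping timer.
; Each timer call of RotateToCamera snaps the Cube's world rotation toward that pawn's CameraComponent, so facing updates in one-second steps rather than every tick.
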(event `self.ReceiveBeginPlay`
  (bind _astwin_stick_pawn (cast `/Game/Blueprints/BP_Gameplay/BP_Player/TwinStickPawn` (`GameplayStatics.GetPlayerPawn` 0)))
  (set `self.PlayerRef` _astwin_stick_pawn)
  (`KismetSystemLibrary.K2_SetTimer` null "RotateToCamera" 1.0 true))

(fn `RotateToCamera`
  (`SceneComponent.K2_SetWorldRotation` (`self.Cube`) (`KismetMathLibrary.FindLookAtRotation` (`SceneComponent.K2_GetComponentLocation` (`self.Cube`)) (`SceneComponent.K2_GetComponentLocation` (`/Game/Blueprints/BP_Gameplay/BP_Player/TwinStickPawn.CameraComponent` (`self.PlayerRef`)))) false false))

(fn `UserConstructionScript`)