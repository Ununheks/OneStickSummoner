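; BP_Enemy is an enemy that scales its stats at spawn, takes damage and awards experience on death.
; BeginPlay bumps ScalingFactor for bosses, scales health, damage, run speed, experience and actor size, then writes movement speeds and roam range to the Blackboard.
; Health and experience grow with the cube of the factor.
; At zero health it destroys itself and adds Experience to PlayerExperience in BP_GameInstance.
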(event `self.ReceiveBeginPlay`
  (bind _returnvalue (`AIBlueprintHelperLibrary.GetBlackboard` null))
  (if (not (not (`self.isBoss?`)))
    (set `self.ScalingFactor` (+ (`self.ScalingFactor`) 1.0)))
  (`self.ApplyScallingToStats`)
  (set `self.CurrentHealth` (`self.MaxHealth`))
  (`BlackboardComponent.SetValueAsFloat` _returnvalue "RunSpeed" (`self.RunSpeed`))
  (`BlackboardComponent.SetValueAsFloat` _returnvalue "WalkSpeed" (`self.WalkSpeed`))
  (`BlackboardComponent.SetValueAsFloat` _returnvalue "RoamRange" (`self.RoamRange`)))

(event `self.ReceiveAnyDamage`
  (params (Damage :type "Float (single-precision)") (DamageType :type "DamageType Object Reference") (InstigatedBy :type "Controller Object Reference") (DamageCauser :type "Actor Object Reference"))
  ;[0.9734 1 0.9671] Getting damaged
  (bind _output_get (set `self.CurrentHealth` (- (`self.CurrentHealth`) Damage)))
  (if (<= _output_get 0.0)
    (`self.K2_DestroyActor`)
    (bind _asbp_game_instance (cast `/Game/Blueprints/BP_GameInstance/BP_GameInstance` (`GameplayStatics.GetGameInstance`)))
    (set `/Game/Blueprints/BP_GameInstance/BP_GameInstance.Player Experience` (+ (`/Game/Blueprints/BP_GameInstance/BP_GameInstance.Player Experience` _asbp_game_instance) (`self.Experience`)) _asbp_game_instance)))

(fn `ApplyScallingToStats`
  (bind _runspeed (`self.RunSpeed`))
  (bind _scalingfactor (`self.ScalingFactor`))
  (set `self.MaxHealth` (* (`self.MaxHealth`) (`KismetMathLibrary.MultiplyMultiply_FloatFloat` _scalingfactor 3.0)))
  (set `self.Damage` (* (`self.Damage`) _scalingfactor))
  (set `self.RunSpeed` (+ _runspeed (* _runspeed (/ _scalingfactor 10.0))))
  (set `self.Experience` (* (`self.Experience`) (`KismetMathLibrary.MultiplyMultiply_FloatFloat` _scalingfactor 3.0)))
  (`self.SetActorScale3D` (* (`self.GetActorScale3D`) _scalingfactor)))

(fn `UserConstructionScript`)