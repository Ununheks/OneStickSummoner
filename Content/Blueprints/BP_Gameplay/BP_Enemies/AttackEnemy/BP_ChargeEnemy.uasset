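; Charge enemy Blueprint, a child enemy class that attacks friendly actors at close range.
; BeginPlay copies its health, speed, range and attack stats from BP_GameInstance for easier development tuning, then calls the parent.
; Attack faces the blackboard's FriendlyActor, damages the first actor in a debug-drawn sphere overlap ahead, and uses a delay as cooldown.
; OnReset swaps the cube's material and prints a debug message.
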(event `/Game/Blueprints/BP_Gameplay/AIInterface.Attack`
  (bind _returnvalue (+ (`self.K2_GetActorLocation`) (* (`KismetMathLibrary.GetForwardVector` (`self.K2_GetActorRotation`)) 200.0)))
  ;[1 1 1] Damaged one enemy in front of a minion
  (`|ExecutionSequence`
    (:`then_0`
      (bind _asactor (cast `Actor` (`BlackboardComponent.GetValueAsObject` (`AIBlueprintHelperLibrary.GetBlackboard` null) "FriendlyActor")))
      (`self.K2_SetActorRotation` (`KismetMathLibrary.FindLookAtRotation` (`self.K2_GetActorLocation`) (`self.K2_GetActorLocation` _asactor))))
    (:`then_1`
      (if (`self.canAttack?`)
        (`KismetSystemLibrary.DrawDebugSphere` _returnvalue 100.0 12 (struct :`R` 1.0 :`A` 1.0))
        (bind _outactors (`KismetSystemLibrary.SphereOverlapActors` _returnvalue 100.0 (`|MakeArray` "ObjectTypeQuery10" :!type "EObjectTypeQuery Enum") null (`|MakeArray` self :!type "Actor Object Reference")))
        (`GameplayStatics.ApplyDamage` (`|GetArrayItem` _outactors) (`self.Damage`))
        (set `self.canAttack?` false)
        (`KismetSystemLibrary.Delay` (/ 1.0 (`self.AttackRate`)))
        (set `self.canAttack?` true)))))

(event `self.ReceiveBeginPlay`
  ;[0.2918 0.2961 0.2961] For development fase for easier setup of variables
  (bind _asbp_game_instance (cast `/Game/Blueprints/BP_GameInstance/BP_GameInstance` (`GameplayStatics.GetGameInstance`)))
  (set `self.Range` (`/Game/Blueprints/BP_GameInstance/BP_GameInstance.ChargeEnemy Range` _asbp_game_instance))
  (set `self.AttackRate` (`/Game/Blueprints/BP_GameInstance/BP_GameInstance.ChargeEnemy AttackRate` _asbp_game_instance))
  (bind _output_get (set `self.MaxHealth` (`/Game/Blueprints/BP_GameInstance/BP_GameInstance.ChargeEnemy MaxHealth` _asbp_game_instance)))
  (set `self.CurrentHealth` _output_get)
  (set `self.RunSpeed` (`/Game/Blueprints/BP_GameInstance/BP_GameInstance.ChargeEnemy RunSpeed` _asbp_game_instance))
  (set `self.WalkSpeed` (`/Game/Blueprints/BP_GameInstance/BP_GameInstance.ChargeEnemy WalkSpeed` _asbp_game_instance))
  (set `self.RoamRange` (`/Game/Blueprints/BP_GameInstance/BP_GameInstance.ChargeEnemy RoamRange` _asbp_game_instance))
  (set `self.RangeOfAgro` (`/Game/Blueprints/BP_GameInstance/BP_GameInstance.ChargeEnemy RangeOfAgro` _asbp_game_instance))
  (`parent.ReceiveBeginPlay`))

(event `self.K2_OnReset`
  (`PrimitiveComponent.SetMaterial` (`self.Cube`) 0 "/Engine/MapTemplates/Materials/BasicAsset01.BasicAsset01")
  (`KismetSystemLibrary.PrintString` "im red dabidudabida"))

(fn `UserConstructionScript`
  (`parent.UserConstructionScript`))