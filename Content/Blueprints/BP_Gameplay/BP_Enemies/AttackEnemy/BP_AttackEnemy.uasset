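; BP_AttackEnemy is an enemy Blueprint that feeds its attack tuning to the AI Blackboard.
; On BeginPlay, after the parent's logic, it writes Range to the AttackRange key and the reciprocal of AttackRate to the AttackRate key, so that key holds an interval rather than a frequency.
; It contains no attack logic of its own, and its construction script only calls the parent.
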(event `self.ReceiveBeginPlay`
  (bind _returnvalue (`AIBlueprintHelperLibrary.GetBlackboard` null))
  (`parent.ReceiveBeginPlay`)
  (`BlackboardComponent.SetValueAsFloat` _returnvalue "AttackRange" (`self.Range`))
  (`BlackboardComponent.SetValueAsFloat` _returnvalue "AttackRate" (/ 1.0 (`self.AttackRate`))))

(fn `UserConstructionScript`
  (`parent.UserConstructionScript`))