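; BP_EnemyTurret is a stationary-style enemy that turns toward and shoots at a TwinStickPawn it sees, and is destroyed when its health runs out.
; PawnSensing sightings rotate the whole actor and spawn a BP_EnemyProjectile, launched by a velocity-change impulse along the Cube's forward vector.
; A boolean gate with a Delay throttles shots, so FireDelay acts as shots per second.
; AnyDamage subtracts from CurrentHealth.
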(event `self.PawnSensing.OnSeePawn`
  (params (Pawn :type "Pawn Object Reference"))
  ;[1 1 1] Wheen sees player
  (bind _astwin_stick_pawn (cast `/Game/TwinStickBP/Blueprints/TwinStickPawn` Pawn))
  (`|ExecutionSequence`
    (:`then_0`
      ;[1 1 1] Turning towards a player
      (`self.K2_SetActorRotation` (`KismetMathLibrary.FindLookAtRotation` (`self.K2_GetActorLocation`) (`self.K2_GetActorLocation` _astwin_stick_pawn))))
    (:`then_1`
      ;[1 1 1] Shooting a projectile towards a player
      (if (`self.SpawnProjectile?`)
        (bind _returnvalue (`|SpawnActorFromClass` "/Game/Blueprints/BP_Gameplay/BP_Projectiles/BP_EnemyProjectile.BP_EnemyProjectile_C" (`SceneComponent.K2_GetComponentToWorld` (`self.ProjectileSpawnLocation`)) "Undefined" "OverrideRootScale" null null))
        (`PrimitiveComponent.AddImpulse` (`/Game/Blueprints/BP_Gameplay/BP_Projectiles/BP_EnemyProjectile.ProjectileMesh` _returnvalue) (* (`SceneComponent.GetForwardVector` (`self.Cube`)) (`self.ProjectileForce`)) "None" true)
        (set `self.SpawnProjectile?` false)
        (`KismetSystemLibrary.Delay` (/ 1.0 (`self.FireDelay`)))
        (set `self.SpawnProjectile?` true)))))

(event `self.ReceiveAnyDamage`
  (params (Damage :type "Float (single-precision)") (DamageType :type "DamageType Object Reference") (InstigatedBy :type "Controller Object Reference") (DamageCauser :type "Actor Object Reference"))
  ;[1 1 1] Getting damaged
  (bind _output_get (set `self.CurrentHealth` (- (`self.CurrentHealth`) Damage)))
  (if (<= _output_get 0.0)
    (set `self.isDead?` true)
    (`self.K2_DestroyActor`)))

(fn `UserConstructionScript`)