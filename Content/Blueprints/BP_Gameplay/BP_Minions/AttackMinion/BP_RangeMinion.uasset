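; Ranged friendly minion that turns toward the enemy stored in its AI blackboard and shoots projectiles at it.
; Attack snaps rotation to the EnemyActor, then spawns BP_FriendlyProjectile with itself as instigator and launches it by impulse along the Cube's forward vector.
; A CanAttack flag and Delay limit fire to AttackRate shots per second.
; BeginPlay copies combat stats and mana cost from BP_GameInstance before calling the parent, a setup meant for easier tuning during development.
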(event `/Game/Blueprints/BP_Gameplay/AIInterface.Attack`
  ;[1 1 1] Shoot a projectile at closest enemy
  (`|ExecutionSequence`
    (:`then_0`
      (bind _asactor (cast `Actor` (`BlackboardComponent.GetValueAsObject` (`AIBlueprintHelperLibrary.GetBlackboard` null) "EnemyActor")))
      (`self.K2_SetActorRotation` (`KismetMathLibrary.FindLookAtRotation` (`self.K2_GetActorLocation`) (`self.K2_GetActorLocation` _asactor))))
    (:`then_1`
      (if (`self.canAttack?`)
        (bind _returnvalue (`|SpawnActorFromClass` "/Game/Blueprints/BP_Gameplay/BP_Projectiles/BP_FriendlyProjectile.BP_FriendlyProjectile_C" (`SceneComponent.K2_GetComponentToWorld` (`self.Projectile Spawn Location`)) "Undefined" "OverrideRootScale" null self))
        (`PrimitiveComponent.AddImpulse` (`/Game/Blueprints/BP_Gameplay/BP_Projectiles/BP_FriendlyProjectile.ProjectileMesh` _returnvalue) (* (`SceneComponent.GetForwardVector` (`self.Cube`)) (`self.ProjectileForce`)) "None" true)
        (set `self.canAttack?` false)
        (`KismetSystemLibrary.Delay` (/ 1.0 (`self.AttackRate`)))
        (set `self.canAttack?` true)))))

(event `self.ReceiveBeginPlay`
  ;[0.2918 0.2961 0.2961] For development fase for easier setup of variables
  (bind _asbp_game_instance (cast `/Game/Blueprints/BP_GameInstance/BP_GameInstance` (`GameplayStatics.GetGameInstance`)))
  (set `self.ProjectileForce` (`/Game/Blueprints/BP_GameInstance/BP_GameInstance.RangeMinion ProjectileForce` _asbp_game_instance))
  (set `self.Range` (`/Game/Blueprints/BP_GameInstance/BP_GameInstance.RangeMinion Range` _asbp_game_instance))
  (set `self.AttackRate` (`/Game/Blueprints/BP_GameInstance/BP_GameInstance.RangeMinion AttackRate` _asbp_game_instance))
  (bind _output_get (set `self.MaxHealth` (`/Game/Blueprints/BP_GameInstance/BP_GameInstance.RangeMinion MaxHealth` _asbp_game_instance)))
  (set `self.CurrentHealth` _output_get)
  (set `self.Damage` (`/Game/Blueprints/BP_GameInstance/BP_GameInstance.RangeMinion Damage` _asbp_game_instance))
  (set `self.ManaCost` (`/Game/Blueprints/BP_GameInstance/BP_GameInstance.RangeMinion ManaCost` _asbp_game_instance))
  (`parent.ReceiveBeginPlay`))

(fn `UserConstructionScript`
  (`parent.UserConstructionScript`))