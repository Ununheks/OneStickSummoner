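; BP_ChargerMinion is an attack minion Blueprint that damages a single enemy in front of it.
; Attack runs a sphere overlap ahead of the minion, ignoring itself, and applies fixed damage to the first actor found, with no empty-result check.
; BeginPlay and construction defer to the parent class.
; Debug output remains: Attack draws a sphere, and Tick prints current health every frame.
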(event `/Game/Blueprints/BP_Gameplay/MinionInterface.Attack`
  (bind _returnvalue (+ (`self.K2_GetActorLocation`) (* (`KismetMathLibrary.GetForwardVector` (`self.K2_GetActorRotation`)) 200.0)))
  ;[1 1 1] Damaged one enemy in front of a minion
  (`KismetSystemLibrary.DrawDebugSphere` _returnvalue)
  (bind _outactors (`KismetSystemLibrary.SphereOverlapActors` _returnvalue 100.0 (`|MakeArray` "ObjectTypeQuery8" :!type "EObjectTypeQuery Enum") null (`|MakeArray` self :!type "Actor Object Reference")))
  (`GameplayStatics.ApplyDamage` (`|GetArrayItem` _outactors) 10.0))

(event `self.ReceiveBeginPlay`
  (`parent.ReceiveBeginPlay`))

(event `self.ReceiveTick`
  (params (DeltaSeconds :type "Float (single-precision)"))
  (`KismetSystemLibrary.PrintString` (`KismetStringLibrary.BuildString_Double` "" "Charger Minion: " (`self.CurrentHealth`))))

(fn `UserConstructionScript`
  (`parent.UserConstructionScript`))