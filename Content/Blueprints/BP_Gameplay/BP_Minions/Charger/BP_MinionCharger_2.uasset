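; Charger minion Blueprint that melee-attacks one enemy and continuously costs the player mana while it is active.
; On BeginPlay it caches the TwinStickPawn player and starts a looping timer that subtracts from its CurrentMana, with no floor check here.
; Attack runs a sphere overlap ahead of the minion, draws a debug sphere there and damages the first actor found, without checking for an empty result.
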(event `/Game/Blueprints/BP_Gameplay/MinionInterface.Attack`
  (bind _returnvalue (+ (`self.K2_GetActorLocation`) (* (`KismetMathLibrary.GetForwardVector` (`self.K2_GetActorRotation`)) 200.0)))
  ;[1 1 1] Damaged one enemy in front of a minion
  (`KismetSystemLibrary.DrawDebugSphere` _returnvalue)
  (bind _outactors (`KismetSystemLibrary.SphereOverlapActors` _returnvalue 100.0 (`|MakeArray` "ObjectTypeQuery8" :!type "EObjectTypeQuery Enum") null (`|MakeArray` self :!type "Actor Object Reference")))
  (`GameplayStatics.ApplyDamage` (`|GetArrayItem` _outactors) 10.0))

(event `self.ReceiveBeginPlay`
  (bind _astwin_stick_pawn (cast `/Game/TwinStickBP/Blueprints/TwinStickPawn` (`GameplayStatics.GetPlayerPawn` 0)))
  (bind _output_get (set `self.PlayerReference` _astwin_stick_pawn))
  (`KismetSystemLibrary.K2_SetTimerDelegate` (delegate `ConsumeMana`) 0.1 true))

(event `ConsumeMana`
  ;[1 1 1] Decrese player mana by 1 every 0.1 sec
  (set `/Game/TwinStickBP/Blueprints/TwinStickPawn.CurrentMana` (- (`/Game/TwinStickBP/Blueprints/TwinStickPawn.CurrentMana` (stale `self.ReceiveBeginPlay` _output_get)) 0.45) (stale `self.ReceiveBeginPlay` _output_get)))

(fn `UserConstructionScript`)